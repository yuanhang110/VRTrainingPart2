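; Extinguisher discharge blob actor: a sphere mesh with optional smoke particles that simulates pressurized spray sticking to what it hits and settling downward.
; On hit, it attaches to the struck component using a weld flag, while Tick lowers mesh and particles at constant speed.
; BeginPlay timelines grow the mesh, particles and collision sphere, then shrink the mesh and fade smoke opacity before destroying the actor.
; A brief particle time-dilation change mimics initial pressure.
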(event Custom|KILL_ME
  ;[1 1 1] Kill this actor
  (Development|SetHiddeninGame (Variables|MyProjectile|GetMesh) true false)
  (Utilities|FlowControl|Delay 0.2)
  (Actor|DestroyActor))

(event EventBeginPlay
  (bind _collisioncomponent (Variables|MyProjectile|GetCollisionComponent))
  (bind _particlesystem (Variables|Default|GetParticleSystem))
  (bind _mesh (Variables|MyProjectile|GetMesh))
  (bind _mesh_2 (Variables|MyProjectile|GetMesh))
  (bind _particlesystem_2 (Variables|Default|GetParticleSystem))
  (bind _meshsmokescale1_2 (Variables|Extinguisher|GetMeshSmokeScale1_2))
  ;[0 0.4084 1] You can change a sphere mesh into another mesh type
  (Components|StaticMesh|SetStaticMesh (Variables|MyProjectile|GetMesh) "/Game/FEPPS/Meshes/SM_Sphere.SM_Sphere")
  ;[1 1 1] Spawn Random Mesh Rot
  (Transformation|SetRelativeRotation (Variables|MyProjectile|GetMesh) (Math|Random|RandomRotator true) false false)
  (Utilities|FlowControl|Sequence
    (:then_0
      ;[1 1 1] View Smoke?
      (if (Variables|Extinguisher|GetActivateSmokeParticle?)
        (Development|SetHiddeninGame _particlesystem_2 false false)
        (else
          (Development|SetHiddeninGame _particlesystem_2 true false))))
    (:then_1
      ;[1 1 1] Increase Spheres & particle size after shooting them
      (bind _newtrack_0 (Timeline|Timeline_0 PlayFromStart)
        (:Update
          (Transformation|SetRelativeScale3D (Variables|MyProjectile|GetMesh) (Math|Vector|MakeVector (* _newtrack_0 _meshsmokescale1_2) (* _newtrack_0 _meshsmokescale1_2) (* _newtrack_0 _meshsmokescale1_2)))
          (Transformation|SetRelativeScale3D (Variables|Default|GetParticleSystem) (Math|Vector|MakeVector (* (* _newtrack_0 _meshsmokescale1_2) _meshsmokescale1_2) (* (* _newtrack_0 _meshsmokescale1_2) _meshsmokescale1_2) (* (* _newtrack_0 _meshsmokescale1_2) _meshsmokescale1_2)))
          (Utilities|FlowControl|Delay 0.5)
          (Collision|SetCollisionEnabled (Variables|MyProjectile|GetCollisionComponent) "QueryOnly"))))
    (:then_2
      ;[1 1 1] Increase also CollisionComponent size (from 20 to 60), together with mesh scale. To increase the 'Hit attach effect', these CollComp scale must be > Mesh scale. The collision is activer for 1 sec.
      (bind _newtrack_0_2 (Timeline|CollisionComponentScale PlayFromStart)
        (:Update
          (Components|Sphere|SetSphereRadius _collisioncomponent (* _newtrack_0_2 _meshsmokescale1_2) true))
        (:Finished
          (Utilities|FlowControl|Delay 0.5)
          (Components|DestroyComponent _collisioncomponent))))
    (:then_3
      ;[1 1 1] Scale decrease from 1 to 0.1 in max10sec (TimeSmokeinAir var), to make all meshes gradually disappear
      (Utilities|FlowControl|Delay 1.0)
      (Utilities|FlowControl|Sequence
        (:then_0
          (bind _newtrack_0_3 (Timeline|Mesh_Smoke_Scale_Decrease SetNewTime)
            (:Update
              (Transformation|SetRelativeScale3D (Variables|MyProjectile|GetMesh) (Math|Vector|MakeVector (* _newtrack_0_3 (Variables|Extinguisher|GetMeshSmokeScale1_2)) (* _newtrack_0_3 (Variables|Extinguisher|GetMeshSmokeScale1_2)) (* _newtrack_0_3 (Variables|Extinguisher|GetMeshSmokeScale1_2)))))))
        (:then_1
          (Timeline|Mesh_Smoke_Scale_Decrease Play))))
    (:then_4
      ;[1 1 1] Removing Weld, meshes will loose the Hit Sticky effect
      (if (not (Variables|Extinguisher|GetActivateSmokeParticle?))
        (Utilities|FlowControl|Delay 1e+01)
        (Variables|Default|SetWeld? false)
        (Rendering|Material|SetMaterial _mesh 0 "/Game/FEPPS/Materials/M_Cyan.M_Cyan")
        (Physics|SetSimulatePhysics _mesh false)
        (Collision|SetCollisionEnabled _mesh "NoCollision")
        ;[1 1 1] Destroy Mesh When smoke mat opacity = 0
        (CallFunction|KILLME :!label _label)))
    (:then_5
      ;[1 1 1] Smoke Material disappears in 20 sec time (Opacity value from 1 to 0)
      (if (Variables|Extinguisher|GetActivateSmokeParticle?)
        (bind _returnvalue (Rendering|Material|CreateDynamicMaterialInstance "/Game/FEPPS/Materials/MI_Smoke_02_Trans_6X6_INST.MI_Smoke_02_Trans_6X6_INST" "None" :!class /Script/Engine.KismetMaterialLibrary))
        (Utilities|FlowControl|Sequence
          (:then_0
            (bind _newtrack_0_4 (Timeline|Mat01_Opacity_1to0 SetNewTime)
              (:Update
                (Rendering|Material|SetScalarParameterValue _returnvalue "Opacity" _newtrack_0_4 :!class /Script/Engine.MaterialInstanceDynamic)
                (Rendering|Material|SetMaterial (Variables|Default|GetParticleSystem) 0 _returnvalue))
              (:Finished
                (goto _label))))
          (:then_1
            (Timeline|Mat01_Opacity_1to0 Play)))))
    (:then_6
      ;[1 1 1] This speeds up the smoke when spawned and after 1sec calms down: useful to simulate smoke pressure at start, then once in the air there is no more pressure and the smokes falls down very slow
      (Variables|/Script/Engine.ParticleSystemComponent|SetCustomTimeDilation _particlesystem (Variables|Extinguisher|GetAirPressureIntensity2_4))
      (Utilities|FlowControl|Delay 0.5)
      (Variables|/Script/Engine.ParticleSystemComponent|SetCustomTimeDilation _particlesystem 1.0))
    (:then_7
      ;[1 1 1] View smoke spheres?
      (if (Variables|Extinguisher|GetHideSmokeSpheres?)
        (Development|SetHiddeninGame _mesh_2 true false)
        (else
          (Development|SetHiddeninGame _mesh_2 false false))))))

(event Collision|EventHit
  (params (MyComp :type Primitive%20Component%20Object%20Reference) (Other :type Actor%20Object%20Reference) (OtherComp :type Primitive%20Component%20Object%20Reference) (bSelfMoved :type Boolean) (HitLocation :type Vector :default "0, 0, 0") (HitNormal :type Vector :default "0, 0, 0") (NormalImpulse :type Vector :default "0, 0, 0") (Hit :type Hit%20Result%20Structure%20%28by%20ref%29))
  ;[1 1 1] Mesh hitting another mesh generate this continuos attach effect, thanks to the 'Weld simulated Bodies' flag=True
  (if (Utilities|IsValid OtherComp)
    (Transformation|AttachComponentToComponent (Variables|MyProjectile|GetMesh) OtherComp "None" "KeepWorld" "KeepWorld" "KeepWorld" (Variables|Default|GetWeld?))
    (Physics|SetSimulatePhysics (Variables|MyProjectile|GetMesh) true)))

(event EventTick
  (params (DeltaSeconds :type Float%20%28single-precision%29))
  (bind _mesh (Variables|MyProjectile|GetMesh))
  (bind _returnvalue (Transformation|GetWorldLocation _mesh))
  (bind (_x _y _z) (Math|Vector|BreakVector _returnvalue))
  ;[1 1 1] This Tick forces 'isolated NonColliding meshes' to fall on the floor smoothly.
  ; Falling speed is 50 and can be changed.
  ; Colliding meshes are already falling thanks to the Hit Weld sim body Enabled (see above comment box)
  ; Particles will follow the sphere mesh movements.
  (Transformation|SetWorldLocation (Variables|Default|GetParticleSystem) (Math|Vector|MakeVector _x _y (- _z (* DeltaSeconds (Variables|Extinguisher|GetForceFallingSpeed10_200)))) false false))

(fn ConstructionScript)