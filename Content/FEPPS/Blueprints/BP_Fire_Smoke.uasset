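; BP_Fire_Smoke is an extinguishable fire, noted as spawned by a bullet explosion, that plays audio and scales up its particles through a timeline on BeginPlay.
; Overlaps on its Extinguisher component by components tagged "extinguisher" decrement FireStrength.
; Once strength drops below zero, a DoOnce ends fire, light and sound, shows enlarged smoke, then destroys the actor after a short delay.
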(event OnComponentBeginOverlap(Extinguisher)
  (params (OverlappedComponent :type Primitive%20Component%20Object%20Reference) (OtherActor :type Actor%20Object%20Reference) (OtherComp :type Primitive%20Component%20Object%20Reference) (OtherBodyIndex :type Integer) (bFromSweep :type Boolean) (SweepResult :type Hit%20Result%20Structure%20%28by%20ref%29))
  (bind _smoke (Variables|Default|GetSmoke))
  ;[1 1 1] When a Smoke sphere mesh overlaps the fire capsule, then start reducing the Fire Strength value
  (if (Components|ComponentHasTag OtherComp "extinguisher")
    (bind _output_get (Variables|Default|SetFireStrength (- (Variables|Default|GetFireStrength) 1.0)))
    ;[1 1 1] When Fire strength is <= 0 then stop fire
    (if (< (Variables|Default|GetFireStrength) 0.0)
      (Utilities|FlowControl|DoOnce false
        (:Completed
          ;[1 1 1] Stop Fire particle and sound, activate smoke particle for 3 sec then destroy all
          (Effects|Particles|Trails|EndTrails (Variables|Default|GetFire))
          (Transformation|SetWorldScale3D _smoke "1.500000,1.500000,1.500000")
          (Development|SetHiddeninGame (Variables|Default|GetPointLight) true false)
          (Effects|Particles|Trails|BeginTrails _smoke "None" "None" "ETrailWidthMode_FromCentre" 0.0)
          (Audio|Components|Audio|Stop (Variables|Default|GetAudio))
          (Utilities|FlowControl|Delay 3.0)
          (Actor|DestroyActor))))))

(event EventBeginPlay
  ;[1 1 1] Start settings: Fire is spawn by bullet explosion
  (Effects|Particles|Trails|EndTrails (Variables|Default|GetSmoke))
  (Effects|Particles|Trails|BeginTrails (Variables|Default|GetFire) "None" "None" "ETrailWidthMode_FromCentre" 0.0)
  (Audio|Components|Audio|Play (Variables|Default|GetAudio) 0.0)
  (bind _newtrack_0 (Timeline|FireScale PlayFromStart)
    (:Update
      (Transformation|SetRelativeScale3D (Variables|Default|GetFire) (Math|Vector|MakeVector _newtrack_0 _newtrack_0 _newtrack_0)))))

(fn ConstructionScript)